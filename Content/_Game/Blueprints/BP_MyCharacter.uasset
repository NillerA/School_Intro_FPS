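; BP_MyCharacter is a character that dies in one hit from any actor tagged "Bullet" and collapses under physics.
; The hit event zeroes Health, and Tick calls Die every frame, which clears the alive flag once and enables physics simulation on the mesh when health runs out.
; The construction script gives each character a random mannequin skeletal mesh.
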(event `self.ReceiveTick`
  (params (DeltaSeconds :type "Float (single-precision)"))
  (`self.Die`))

(event `Die`
  ;[1 1 1] Death when out of health
  (if (and (`self.IsAlvive`) (<= (`self.health`) 0))
    (set `self.IsAlvive` false)
    (`PrimitiveComponent.SetSimulatePhysics` (`self.Mesh`) true)))

(event `self.ReceiveHit`
  (params (MyComp :type "PrimitiveComponent Object Reference") (Other :type "Actor Object Reference") (OtherComp :type "PrimitiveComponent Object Reference") (bSelfMoved :type Boolean) (HitLocation :type "Vector Structure") (HitNormal :type "Vector Structure") (NormalImpulse :type "Vector Structure") (Hit :type "HitResult Structure (by ref)"))
  (if (`self.ActorHasTag` Other "Bullet")
    (set `self.health` 0)))

(fn `UserConstructionScript`
  (bind _array (`|MakeArray` "/Game/Characters/Mannequin_UE4/Meshes/SK_Mannequin.SK_Mannequin" "/Game/Characters/Mannequins/Meshes/SKM_Manny.SKM_Manny" "/Game/Characters/Mannequins/Meshes/SKM_Quinn.SKM_Quinn" :!type "SkeletalMesh Object Reference"))
  (`SkeletalMeshComponent.SetSkeletalMeshAsset` (`self.Mesh`) (`|GetArrayItem` _array (`KismetMathLibrary.RandomInteger` (`KismetArrayLibrary.Array_Length` _array)))))